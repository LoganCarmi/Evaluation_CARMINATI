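; BP_Enemy is an enemy Blueprint that turns to face the player while the player is inside its detection zone.
; DetectionZone overlap events set IsAttacking when a BP_MainCharacter enters and clear it when one leaves.
; While IsAttacking is true, Tick looks up the character with GetActorOfClass and snaps rotation toward it, keeping pitch at zero.
; Attack mode contains no damage or movement logic, only this facing behavior.
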(event OnComponentBeginOverlap(DetectionZone)
  (params (OverlappedComponent :type Primitive%20Component%20Object%20Reference) (OtherActor :type Actor%20Object%20Reference) (OtherComp :type Primitive%20Component%20Object%20Reference) (OtherBodyIndex :type Integer) (bFromSweep :type Boolean) (SweepResult :type Hit%20Result%20Structure%20%28by%20ref%29))
  ;[1 1 1] When Player in Range, activate Attack Mode
  (Utilities|Casting|CastToBP_MainCharacter OtherActor)
  (Variables|Default|SetbIsAttacking true))

(event OnComponentEndOverlap(DetectionZone)
  (params (OverlappedComponent :type Primitive%20Component%20Object%20Reference) (OtherActor :type Actor%20Object%20Reference) (OtherComp :type Primitive%20Component%20Object%20Reference) (OtherBodyIndex :type Integer))
  ;[1 1 1] When Player leaves the range, deactivate the Attack Mode
  (Utilities|Casting|CastToBP_MainCharacter OtherActor)
  (Variables|Default|SetbIsAttacking false))

(event EventTick
  (params (DeltaSeconds :type Float%20%28single-precision%29))
  ;[1 0 0] Event Tick : Always face the player when in Attack Mode
  (if (Variables|Default|GetbIsAttacking)
    (bind _returnvalue (Actor|GetActorOfClass "/Game/EvalOpti/Game/Blueprints/BP_MainCharacter.BP_MainCharacter_C"))
    (Transformation|SetActorRotation (Math|Rotator|MakeRotator (.Roll (Math|Rotator|BreakRotator (Math|Rotator|FindLookatRotation (Transformation|GetActorLocation) (Transformation|GetActorLocation _returnvalue)))) 0.0 (.Yaw (Math|Rotator|BreakRotator (Math|Rotator|FindLookatRotation (Transformation|GetActorLocation) (Transformation|GetActorLocation _returnvalue))))))))

(fn ConstructionScript)