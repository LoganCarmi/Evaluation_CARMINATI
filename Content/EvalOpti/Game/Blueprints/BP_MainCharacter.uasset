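; Player character Blueprint with Enhanced Input movement, camera look, a lock-on camera and a basic attack gate.
; Lock-on toggles targeting of the closest BP_Enemy within detection range and spawns a BP_LockArrow above it.
; While locked, look input is ignored and Tick rotates the controller from the spring arm toward the target.
; Attack only sets IsAttacking and disables player input for a fixed delay.
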(event Input|EnhancedActionEvents|EnhancedInputActionIA_Look
  (params (ActionValue :type Vector%202D%20Structure) (ElapsedSeconds :type Float%20%28double-precision%29) (TriggeredSeconds :type Float%20%28double-precision%29) (InputAction :type Input%20Action%20Object%20Reference :default "/Game/EvalOpti/Inputs/Actions/IA_Look.IA_Look"))
  (bind (_x _y) (Math|Vector2D|BreakVector2D ActionValue))
  ;[1 0 1] Camera Movement
  (if (not (Variables|Default|GetbIsTargetLocked))
    (Pawn|Input|AddControllerYawInput _x)
    (Pawn|Input|AddControllerPitchInput (* _y -1.0))))

(event Input|EnhancedActionEvents|EnhancedInputActionIA_Move
  (params (ActionValue :type Vector%202D%20Structure) (ElapsedSeconds :type Float%20%28double-precision%29) (TriggeredSeconds :type Float%20%28double-precision%29) (InputAction :type Input%20Action%20Object%20Reference :default "/Game/EvalOpti/Inputs/Actions/IA_Move.IA_Move"))
  (bind (_x _y) (Math|Vector2D|BreakVector2D ActionValue))
  (bind _returnvalue (Pawn|GetControlRotation :!class /Script/Engine.Pawn))
  ;[0 0 1] Player Movement
  (Variables|Default|SetPlayerMovement ActionValue)
  (Pawn|Input|AddMovementInput (Math|Vector|GetRightVector (Math|Rotator|MakeRotator (.roll _returnvalue) 0.0 (.yaw _returnvalue))) _x false)
  (Pawn|Input|AddMovementInput (Math|Vector|GetForwardVector (Math|Rotator|MakeRotator 0.0 0.0 (.yaw (Pawn|GetControlRotation :!class /Script/Engine.Pawn)))) _y false))

(event Input|EnhancedActionEvents|EnhancedInputActionIA_Lock
  (params (ActionValue :type Boolean) (ElapsedSeconds :type Float%20%28double-precision%29) (TriggeredSeconds :type Float%20%28double-precision%29) (InputAction :type Input%20Action%20Object%20Reference :default "/Game/EvalOpti/Inputs/Actions/IA_Lock.IA_Lock"))
  ;[0 1 1] Lock Camera
  (:Started
    (CallFunction|ToggleLock-On)))

(event Input|EnhancedActionEvents|EnhancedInputActionIA_Attack
  (params (ActionValue :type Boolean) (ElapsedSeconds :type Float%20%28double-precision%29) (TriggeredSeconds :type Float%20%28double-precision%29) (InputAction :type Input%20Action%20Object%20Reference :default "/Game/EvalOpti/Inputs/Actions/IA_Attack.IA_Attack"))
  ;[1 0 1] Attack : Disable inputs while attacking
  (if (not (Variables|Default|GetbIsAttacking))
    (Input|DisableInput (Game|GetPlayerController 0))
    (Variables|Default|SetbIsAttacking true)
    (Utilities|FlowControl|Delay 1.0)
    (Variables|Default|SetbIsAttacking false)
    (Input|EnableInput (Game|GetPlayerController 0))))

(event EventBeginPlay
  ;[1 0 0] Begin Play : InputMapping
  (bind _asplayer_controller (Utilities|Casting|CastToPlayerController (Pawn|GetController)))
  (Input|AddMappingContext (PlayerController|LocalPlayerSubsystems|GetEnhancedInputLocalPlayerSubsystem _asplayer_controller) "/Game/EvalOpti/Inputs/Mappings/IMC_MainCharacter.IMC_MainCharacter" 0 "(bIgnoreAllPressedKeysUntilRelease=True,bForceImmediately=False,bNotifyUserSettings=False)"))

(event EventTick
  (params (DeltaSeconds :type Float%20%28single-precision%29))
  ;[1 0.3 0] Event Tick : Set Controller Rotation if target locked
  (if (Variables|Default|GetbIsTargetLocked)
    (Pawn|SetControlRotation (Pawn|GetController) (Math|Rotator|FindLookatRotation (Transformation|GetWorldLocation (Variables|Default|GetSpringArm)) (Transformation|GetActorLocation (Variables|Default|GetCurrentLockTarget))))))

(fn ConstructionScript)

(fn ToggleLock-On
  (if (Variables|Default|GetbIsTargetLocked)
    ;[0 1 0] Return to default parameters
    (Variables|Default|SetCurrentLockTarget 0)
    (Variables|/Script/Engine.SpringArmComponent|SetbUsePawnControlRotation (Variables|Default|GetSpringArm) true)
    (Variables|Default|SetbIsTargetLocked false)
    (Actor|DestroyActor (Variables|Default|GetLockArrow))
    (Variables|Default|SetLockArrow 0)
    (else
      (bind _closestenemy (CallFunction|GetClosestEnemy))
      (Utilities|IsValid _closestenemy
        (:Is%20Valid
          (bind _output_get (Variables|Default|SetCurrentLockTarget _closestenemy))
          (Variables|/Script/Engine.SpringArmComponent|SetbUsePawnControlRotation (Variables|Default|GetSpringArm) false)
          (Variables|Default|SetbIsTargetLocked true)
          ;[1 1 0] Spawn an Lock Arrow with an Z Offset above
          (bind _returnvalue (Game|SpawnActorfromClass "/Game/EvalOpti/Game/Blueprints/BP_LockArrow.BP_LockArrow_C" (Math|Transform|MakeTransform (+ (.Location (Math|Transform|BreakTransform (Transformation|GetActorTransform _output_get))) (Math|Vector|MakeVector 0.0 0.0 (* (.X (Math|Vector|BreakVector (.Scale (Math|Transform|BreakTransform (Transformation|GetActorTransform _output_get))))) 2e+02))) (.Rotation (Math|Transform|BreakTransform (Transformation|GetActorTransform _output_get))) (.Scale (Math|Transform|BreakTransform (Transformation|GetActorTransform _output_get)))) "AlwaysSpawn" "MultiplyWithRoot" _output_get 0))
          (Variables|Default|SetLockArrow _returnvalue))))))

(fn GetClosestEnemy
  (bind _self self)
  (bind _outactors (Actor|GetAllActorsOfClass "/Game/EvalOpti/Game/Blueprints/BP_Enemy.BP_Enemy_C"))
  (for _array_element _outactors
    ;[1 1 1] Check if Enemy is in range
    (if (< (Transformation|GetDistanceTo _array_element self) (Variables|Default|GetMinimumDetectionRange))
      (Utilities|IsValid (LocalVariables|GetClosestEnemyRef)
        (:Is%20Valid
          (if (> (Transformation|GetDistanceTo _self (LocalVariables|GetClosestEnemyRef)) (Transformation|GetDistanceTo _self _array_element))
            (LocalVariables|SetClosestEnemyRef _array_element)))
        (:Is%20Not%20Valid
          (LocalVariables|SetClosestEnemyRef _array_element)))))
  (return (LocalVariables|GetClosestEnemyRef)))